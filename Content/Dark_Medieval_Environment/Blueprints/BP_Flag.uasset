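; BP_Flag is a medieval-environment flag actor whose skeletal-mesh cloth flutters in randomized wind.
; The construction script assigns the mesh and writes the flag color to custom primitive data.
; From BeginPlay, a delay loop periodically feeds the Chaos clothing interactor a new wind velocity based on actor forward, with random angle and speed.
; The rotation axis is a zero vector, so the angle does not truly turn the wind direction.
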(event EventBeginPlay
  (bind _output_get (Variables|Default|SetFlag%20SkeletalMesh (Variables|Default|GetFlag%20SkeletalMesh)))
  (bind _aschaos_clothing_interactor (Utilities|Casting|CastToChaosClothingInteractor (Class|ClothingSimulationInteractor|GetClothingInteractor (Class|SkeletalMeshComponent|GetClothingSimulationInteractor _output_get) (Variables|Components|GetClothing%20Asset%20Name))))
  (Class|ChaosClothingInteractor|SetWind _aschaos_clothing_interactor "(X=0.070000,Y=0.500000)" "(X=0.070000,Y=0.500000)" 1e-06 (* (Math|Vector|RotateVectorAroundAxis (Transformation|GetActorForwardVector) (Math|Random|RandomFloatinRange 1.3e+02 3e+02) "0, 0, 0") (Math|Random|RandomFloatinRange (Variables|Components|GetWind%20Velocity%20Min) (Variables|Components|GetWind%20Velocity%20Max))) :!label _label)
  (Utilities|FlowControl|Delay (Variables|Components|GetWind%20Update%20in%20Seconds))
  (goto _label))

(fn ConstructionScript
  (bind _flag_skeletalmesh (Variables|Default|GetFlag%20SkeletalMesh))
  (Components|SkeletalMesh|SetSkeletalMeshAsset _flag_skeletalmesh (Variables|Components|GetFlag%20Skeletal%20Mesh))
  (Rendering|Material|SetCustomPrimitiveDataVector3 _flag_skeletalmesh 0 (Variables|Components|GetFlag%20Color%20%28Custom%20Primitive%20Data%29)))